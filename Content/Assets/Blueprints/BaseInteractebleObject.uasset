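; Base Blueprint for interactable objects that shows an interaction widget while a player interacts with it.
; Interact calls its parent, then creates an InteractWidgetBP, stores it and adds it to the viewport; StopInteract calls its parent and removes that widget.
; Interaction passes the player to BeginInteract, an empty hook here, and returns false.
; The event graph and construction script add no behavior of their own.
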(event EventBeginPlay
  (|CallParentFunction) ; This node is disabled and will not be called.\nDrag off pins to build functionality.
)

(event Collision|EventActorBeginOverlap
  (params (OtherActor :type Actor%20Object%20Reference)))

(event EventTick
  (params (DeltaSeconds :type Float%20%28single-precision%29)))

(fn ConstructionScript
  (|CallParentFunction))

(fn StopInteract
  (params (PlayerRef :type Scavanger%20Object%20Reference))
  (|CallParentFunction PlayerRef)
  (Widget|RemovefromParent (Variables|Default|GetWidget)))

(fn Interact
  (params (PlayerRef :type Scavanger%20Object%20Reference))
  (|CallParentFunction PlayerRef)
  (bind _returnvalue (Game|ConstructObjectfromClass "/Game/Assets/Blueprints/InteractWidgetBP.InteractWidgetBP_C"))
  (bind _output_get (Variables|Default|SetWidget _returnvalue))
  (UserInterface|Viewport|AddtoViewport _output_get 0))

(fn BeginInteract
  (params (PlayerRef :type Scavanger%20Object%20Reference)))

(fn Interaction
  (params (PlayerRef :type Scavanger%20Object%20Reference))
  (CallFunction|BeginInteract PlayerRef)
  (return false))